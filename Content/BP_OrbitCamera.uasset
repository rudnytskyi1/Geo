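; Orbit camera that rotates and zooms a spring arm through Enhanced Input, adding its own mapping context on BeginPlay.
; Holding the rotate input hides the cursor, switches to game-only input and lets look input turn the arm with clamped pitch.
; Zoom input adds velocity that Tick applies to the clamped arm length and damps toward zero.
; While zooming, yaw and pitch speeds are remapped from arm length, making rotation slower up close.
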(event `EnhancedInput|/Game/IA_Look`
  (params (ActionValue :type "Vector2D Structure") (ElapsedSeconds :type "Float (double-precision)") (TriggeredSeconds :type "Float (double-precision)") (InputAction :type "InputAction Object Reference" :default "/Game/IA_Look.IA_Look"))
  (bind (_x _y) (`KismetMathLibrary.BreakVector2D` ActionValue))
  (bind _springarm (`self.SpringArm`))
  (bind (_relativerotation_roll _relativerotation_pitch _relativerotation_yaw) (`KismetMathLibrary.BreakRotator` (`SceneComponent.RelativeRotation` _springarm)))
  (:`Triggered`
    (if (`self.IsRotating`)
      (`SceneComponent.K2_SetRelativeRotation` _springarm (`KismetMathLibrary.MakeRotator` 0.0 (`KismetMathLibrary.FClamp` (+ _relativerotation_pitch (* _y (`self.PitchSpeed`))) -85.0 85.0) (+ _relativerotation_yaw (* _x (`self.YawSpeed`)))) false false))))

(event `self.ReceiveBeginPlay`
  (`EnhancedInputSubsystemInterface.AddMappingContext` (pcsubsystem `EnhancedInputLocalPlayerSubsystem` (`GameplayStatics.GetPlayerController` 0)) "/Game/IMC_OrbitCamera.IMC_OrbitCamera" 0 (struct)))

(event `EnhancedInput|/Game/IA_Rotate`
  (params (ActionValue :type Boolean) (ElapsedSeconds :type "Float (double-precision)") (TriggeredSeconds :type "Float (double-precision)") (InputAction :type "InputAction Object Reference" :default "/Game/IA_Rotate.IA_Rotate"))
  (bind _returnvalue (`GameplayStatics.GetPlayerController` 0))
  (:`Triggered`
    (set `self.IsRotating` true)
    (`WidgetBlueprintLibrary.SetInputMode_GameOnly` _returnvalue)
    (set `PlayerController.bShowMouseCursor` false _returnvalue))
  (:`Completed`
    (set `self.IsRotating` false)
    (set `PlayerController.bShowMouseCursor` true _returnvalue)
    (`WidgetBlueprintLibrary.SetInputMode_GameAndUIEx` _returnvalue null "DoNotLock" false)))

(event `self.ReceiveTick`
  (params (DeltaSeconds :type "Float (single-precision)"))
  (bind _zoomvelocity (`self.ZoomVelocity`))
  (bind _springarm (`self.SpringArm`))
  (bind _returnvalue (`KismetMathLibrary.MapRangeClamped` (`SpringArmComponent.TargetArmLength` (`self.SpringArm`)) (`self.MinArmLength`) (`self.MaxArmLength`) 0.2 1.25))
  (if (> (`KismetMathLibrary.Abs` _zoomvelocity) 0.01)
    (set `SpringArmComponent.TargetArmLength` (`KismetMathLibrary.FClamp` (+ (`SpringArmComponent.TargetArmLength` _springarm) (* (`self.ZoomVelocity`) DeltaSeconds)) (`self.MinArmLength`) (`self.MaxArmLength`)) _springarm)
    (set `self.ZoomVelocity` (`KismetMathLibrary.FInterpTo` _zoomvelocity 0.0 DeltaSeconds (`self.ZoomDamping`)))
    (set `self.YawSpeed` _returnvalue)
    (set `self.PitchSpeed` _returnvalue)))

(event `EnhancedInput|/Game/IA_Zoom`
  (params (ActionValue :type "Float (double-precision)") (ElapsedSeconds :type "Float (double-precision)") (TriggeredSeconds :type "Float (double-precision)") (InputAction :type "InputAction Object Reference" :default "/Game/IA_Zoom.IA_Zoom"))
  (:`Triggered`
    (set `self.ZoomVelocity` (+ (`self.ZoomVelocity`) (* ActionValue (`self.ZoomImpulse`))))))

(fn `UserConstructionScript`)